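; BP_BossAI is a boss AI actor that detects hero characters and performs melee-or-other montage attacks on a target.
; A Sphere overlap writes the hero to the AI controller's Blackboard "Target" key and clears it when that target leaves.
; The ATK_01 event yaws the boss toward a valid target, then plays a random AttackArray montage, with a random range that includes the out-of-bounds Length index.
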(event OnComponentBeginOverlap(Sphere)
  (params (OverlappedComponent :type Primitive%20Component%20Object%20Reference) (OtherActor :type Actor%20Object%20Reference) (OtherComp :type Primitive%20Component%20Object%20Reference) (OtherBodyIndex :type Integer) (bFromSweep :type Boolean) (SweepResult :type Hit%20Result%20Structure%20%28by%20ref%29))
  ;[1 1 1] Get, Set, Clear Target
  (if (!= OtherActor self)
    (bind _asbp_hero_character (Utilities|Casting|CastToBP_HeroCharacter OtherActor))
    (CallFunction|SetTarget _asbp_hero_character)))

(event OnComponentEndOverlap(Sphere)
  (params (OverlappedComponent :type Primitive%20Component%20Object%20Reference) (OtherActor :type Actor%20Object%20Reference) (OtherComp :type Primitive%20Component%20Object%20Reference) (OtherBodyIndex :type Integer))
  ;[1 1 1] Get, Set, Clear Target
  (if (== OtherActor (CallFunction|GetTarget))
    (CallFunction|ClearTarget)))

(event Custom|ATK_01
  (params (Target :type Actor%20Object%20Reference))
  (bind _attackarray (Variables|Default|GetAttackArray))
  ;[1 1 1] Attack
  (Utilities|FlowControl|Sequence
    (:then_0
      (Utilities|IsValid Target
        (:Is%20Valid
          (Transformation|SetActorRotation (Math|Rotator|MakeRotator 0.0 0.0 (.yaw (Math|Rotator|FindLookatRotation (Transformation|GetActorLocation) (Transformation|GetActorLocation Target))))))))
    (:then_1
      (Animation|PlayAnimMontage (Utilities|Array|Get(acopy) _attackarray (Math|Random|RandomIntegerinRange 0 (Utilities|Array|Length _attackarray))) 1.0 "None"))))

(fn ConstructionScript)

(fn SetTarget
  (params (newTarget :type Actor%20Object%20Reference))
  (AI|Components|Blackboard|SetValueasObject (AI|GetBlackboard (AI|GetAIController self)) (Utilities|Name|MakeLiteralName "Target") newTarget))

(fn GetTarget
  (return (.AsActor (Utilities|Casting|CastToActor (AI|Components|Blackboard|GetValueasObject (AI|GetBlackboard (AI|GetAIController self)) (Utilities|Name|MakeLiteralName "Target"))))))

(fn ClearTarget
  (AI|Components|Blackboard|ClearValue (AI|GetBlackboard (AI|GetAIController self)) (Utilities|Name|MakeLiteralName "Target")))