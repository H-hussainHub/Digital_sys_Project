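; Base enemy AI character that roams around its spawn point and fights a player target once one is set.
; AIMoveTo drives roaming and chasing; in combat it faces the target, taunts if distant, then loops chase and attack.
; Attacks are picked by distance with random montages, whose length paces the loop.
; Authority-only sphere overlaps apply damage by attack type, while ClearTarget and DoRangeAttack are empty stubs.
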(event OnComponentBeginOverlap(MeleeSphere)
  (params (OverlappedComponent :type Primitive%20Component%20Object%20Reference) (OtherActor :type Actor%20Object%20Reference) (OtherComp :type Primitive%20Component%20Object%20Reference) (OtherBodyIndex :type Integer) (bFromSweep :type Boolean) (SweepResult :type Hit%20Result%20Structure%20%28by%20ref%29))
  (Networking|SwitchHasAuthority
    (:Authority
      (if (Actor|ActorHasTag OtherActor "Player")
        (CallFunction|FGetDamage OtherActor)))))

(event Custom|Multi_PlayMontage
  (params (InSkeletalMeshComponent :type Skeletal%20Mesh%20Component%20Object%20Reference) (MontageToPlay :type Anim%20Montage%20Object%20Reference) (StartingSection :type Name))
  (Animation|Montage|PlayMontage InSkeletalMeshComponent MontageToPlay 1.0 0.0 StartingSection))

(event EventBeginPlay
  ;[1 1 1] Set Movement State and AI Roaming
  (CallFunction|FMovementState "NewEnumerator1")
  (Variables|Default|SetStartingLocation (Transformation|GetActorLocation))
  (Utilities|FlowControl|Delay 1.0)
  (CallFunction|SetRoaming))

(event EventCheckforTaunt
  (bind _tauntmontage (Variables|EnemyInfo|GetTauntMontage))
  (bind _output (CallFunction|FGetMontage _tauntmontage))
  ;[1 1 1] Taunt/Aggro
  (AI|Navigation|StopMovement (Pawn|GetController))
  (if (>= (Transformation|GetDistanceTo self (Variables|Default|GetPlayerTarget)) 8e+02)
    (CallFunction|MultiPlayMontage (Variables|Character|GetMesh) _output "None")
    (bind _returnvalue (Animation|GetPlayLength _output))
    (Utilities|FlowControl|Delay _returnvalue)
    (CallFunction|ChasePlayer)
    (else
      (CallFunction|ChasePlayer))))

(event EventDoRangeAttack)

(event EventClearTarget)

(event EventSetRoaming
  ;[1 1 1] Set Movement State and AI Roaming
  (if (and (not (Variables|Default|GetIsRoaming)) (not (Variables|Default|GetIsCombat)))
    (AI|AIMoveTo self (.RandomLocation (AI|Navigation|GetRandomReachablePointinRadius (Variables|Default|GetStartingLocation) 1.2e+03 0 0)) 0 2.5e+02 false
      (:then
        (Variables|Default|SetIsRoaming true))
      (:OnSuccess
        (Variables|Default|SetIsRoaming false)
        (Utilities|FlowControl|Delay 5.0)
        (CallFunction|SetRoaming))
      (:OnFail
        (CallFunction|ClearTarget)))))

(event EventSetPlayerTarget
  (params (Target :type Actor%20Object%20Reference))
  ;[1 1 1] Target and Rotate to player
  (Variables|Default|SetPlayerTarget Target)
  (Variables|Default|SetIsCombat true)
  (Actor|Tick|SetActorTickEnabled true)
  (Variables|Default|SetStartCombatLocation (Transformation|GetActorLocation))
  (CallFunction|FMovementState "NewEnumerator2")
  (CallFunction|CheckforTaunt))

(event EventTick
  (params (DeltaSeconds :type Float%20%28single-precision%29))
  ;[1 1 1] Target and Rotate to player
  (if (Variables|Default|GetIsCombat)
    (Variables|Default|GetPlayerTarget
      (:then
        (Transformation|SetActorRotation (Math|Rotator|MakeRotator 0.0 0.0 (.yaw (Math|Rotator|FindLookatRotation (Transformation|GetActorLocation) (Transformation|GetActorLocation (Variables|Default|GetPlayerTarget)))))))
      (:else))))

(event EventChasePlayer
  ;[1 1 1] Chasing Player
  (if (Variables|Default|GetIsCombat)
    (AI|AIMoveTo self "0, 0, 0" (Variables|Default|GetPlayerTarget) 5e+01 true
      (:OnSuccess
        (CallFunction|RunAttackChoices)))))

(event EventRunAttackChoices
  (if (Variables|Default|GetIsCombat)
    (bind _playertarget (Variables|Default|GetPlayerTarget)
      (:then
        (bind _dead (Class|INTHeroCharacter|IsDead(Message) _playertarget))
        (if (not _dead)
          (bind _length (CallFunction|FPickAttack (Transformation|GetDistanceTo self (Variables|Default|GetPlayerTarget))))
          (Utilities|FlowControl|Delay (+ _length 0.5))
          (CallFunction|ChasePlayer)
          (else
            (CallFunction|ClearTarget))))
      (:else
        (CallFunction|ClearTarget)))))

(event EventSetMeleeCollision
  (params (State :type Boolean))
  (if State
    (Collision|SetCollisionEnabled (Variables|Default|GetMeleeSphere) "QueryOnly")
    (else
      (Collision|SetCollisionEnabled (Variables|Default|GetMeleeSphere) "QueryOnly"))))

(event EventDoSphereOverlap
  (bind _returnvalue (Transformation|GetActorLocation))
  (bind _returnvalue_2 (Transformation|GetActorForwardVector))
  (bind _returnvalue_3 (* _returnvalue_2 2e+02))
  (bind _returnvalue_4 (+ _returnvalue _returnvalue_3))
  (Networking|SwitchHasAuthority
    (:Authority
      (bind _outactors (Collision|SphereOverlapActors _returnvalue_4 1e+02 (Utilities|Array|MakeArray "ObjectTypeQuery3") 0 (Utilities|Array|MakeArray self)))
      (Rendering|Debug|DrawDebugSphere _returnvalue_4 1e+02 12 "(R=1.000000,G=0.104167,B=0.104167,A=1.000000)" 2.0 1.0)
      (for _array_element _outactors
        (if (Actor|ActorHasTag _array_element "Player")
          (CallFunction|FGetDamage _array_element))))))

(fn ConstructionScript
  (|CallParentFunction))

(fn FMovementState
  (params (State :type E_AIMovementState%20Enum :default "NewEnumerator0"))
  (bind _walkspeed (Variables|EnemyInfo|GetWalkSpeed))
  (Variables|/Script/Engine.CharacterMovementComponent|SetMaxWalkSpeed (Variables|Character|GetCharacterMovement) (Utilities|Select :Index State :NewEnumerator0 0.0 :NewEnumerator1 _walkspeed :NewEnumerator2 (* _walkspeed (Variables|EnemyInfo|GetSpeedMultiplier)))))

(fn FPickAttack
  (params (DistanceToPlayer :type Float%20%28single-precision%29))
  (bind _rangeattackmontages (Variables|EnemyInfo|GetRangeAttackMontages))
  (bind _lightattackmontages (Variables|EnemyInfo|GetLightAttackMontages))
  (bind _heavyattackmontages (Variables|EnemyInfo|GetHeavyAttackMontages))
  (bind _specialattackmontages (Variables|EnemyInfo|GetSpecialAttackMontages))
  (bind _output (CallFunction|FGetMontage _specialattackmontages))
  (bind _output_2 (CallFunction|FGetMontage _heavyattackmontages))
  (bind _output_3 (CallFunction|FGetMontage _rangeattackmontages))
  (bind _output_4 (CallFunction|FGetMontage _lightattackmontages))
  (if (<= DistanceToPlayer (Variables|EnemyInfo|GetMeleeDistance))
    (if (CallFunction|FPercentage 6e+01)
      (Variables|Default|SetAttackTypes "NewEnumerator0")
      (CallFunction|MultiPlayMontage (Variables|Character|GetMesh) _output_4 "None")
      (bind _returnvalue (Animation|GetPlayLength _output_4))
      (return _returnvalue)
      (else
        (Variables|Default|SetAttackTypes "NewEnumerator1")
        (CallFunction|MultiPlayMontage (Variables|Character|GetMesh) _output_2 "None")
        (bind _returnvalue_2 (Animation|GetPlayLength _output_2))
        (return _returnvalue_2)))
    (elif (<= DistanceToPlayer (Variables|EnemyInfo|GetRangedDistance))
      (Variables|Default|SetAttackTypes "NewEnumerator3")
      (CallFunction|MultiPlayMontage (Variables|Character|GetMesh) _output "None")
      (bind _returnvalue_3 (Animation|GetPlayLength _output))
      (return _returnvalue_3)
      (else
        (Variables|Default|SetAttackTypes "NewEnumerator2")
        (CallFunction|MultiPlayMontage (Variables|Character|GetMesh) _output_3 "None")
        (bind _returnvalue_4 (Animation|GetPlayLength _output_3))
        (return _returnvalue_4)))))

(fn FGetMontage
  (params (Montages :type Array%20of%20Anim%20Montage%20Object%20References))
  (return (Utilities|Array|Get(acopy) Montages (Math|Random|RandomIntegerinRange 0 (- (Utilities|Array|Length Montages) 1)))))

(fn FGetDamage
  (params (HitPlayer :type Actor%20Object%20Reference))
  (Game|Damage|ApplyDamage HitPlayer (Utilities|Select :Index (Variables|Default|GetAttackTypes) :NewEnumerator0 (Variables|EnemyInfo|GetLightAttackDamage) :NewEnumerator1 (Variables|EnemyInfo|GetHeavyAttackDamage) :NewEnumerator2 (Variables|EnemyInfo|GetRangeAttackDamage) :NewEnumerator3 (Variables|EnemyInfo|GetSpecialAttackDamage)) 0 self "/Script/Engine.DamageType"))

(fn FPercentage
  (params (Percent :type Float%20%28single-precision%29))
  (return (select (== Percent 0.0) false (<= (Math|Random|RandomFloatinRange 0.0 1e+02) Percent))))

(fn FGetAttackType
  (return (Variables|Default|GetAttackTypes)))

(fn FGetCombatState
  (return (Variables|Default|GetIsCombat)))

(fn FGetPlayerTarget
  (return (Variables|Default|GetPlayerTarget)))