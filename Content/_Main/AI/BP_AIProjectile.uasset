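; BP_AIProjectile is a projectile fired by AI that damages players on overlap.
; On the server, the sphere overlap applies damage to Player-tagged actors with the owner as causer, then destroys itself.
; It passes through Enemy-tagged actors and destroys itself on any other overlap.
; On destruction after a hit, it spawns the hit emitter at its location through a Multi_SpawnFX event.
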(event OnComponentBeginOverlap(Sphere)
  (params (OverlappedComponent :type Primitive%20Component%20Object%20Reference) (OtherActor :type Actor%20Object%20Reference) (OtherComp :type Primitive%20Component%20Object%20Reference) (OtherBodyIndex :type Integer) (bFromSweep :type Boolean) (SweepResult :type Hit%20Result%20Structure%20%28by%20ref%29))
  (Networking|SwitchHasAuthority
    (:Authority
      (if (Actor|ActorHasTag OtherActor "Player")
        (Variables|Default|SetHit true)
        (Game|Damage|ApplyDamage OtherActor (Variables|Default|GetDamage) 0 (Components|GetOwner) "/Script/Engine.DamageType")
        (Actor|DestroyActor)
        (elif (not (Actor|ActorHasTag OtherActor "Enemy"))
          (Variables|Default|SetHit true)
          (Actor|DestroyActor))))))

(event Custom|Multi_SpawnFX
  (params (EmitterTemplate :type Particle%20System%20Object%20Reference) (Location :type Vector))
  (Effects|SpawnEmitteratLocation EmitterTemplate Location))

(event EventDestroyed
  (if (Variables|Default|GetHit)
    (CallFunction|MultiSpawnFX (Variables|Default|GetHitEmitter) (Transformation|GetActorLocation))))

(fn ConstructionScript)