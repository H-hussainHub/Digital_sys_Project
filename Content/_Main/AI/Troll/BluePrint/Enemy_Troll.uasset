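; Troll enemy AI character with heavy, charge and ranged vomit attacks against players.
; While in combat, ChasePlayer loops on a delay, picking attacks by target distance, moving toward the target and running attack choices on arrival.
; Authority-only sphere overlaps damage tagged players and launch them upward along the player-to-troll direction, with debug spheres drawn.
; The ranged attack spawns a vomit projectile on the authority.
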(event EventDoRangeAttack
  (Networking|SwitchHasAuthority
    (:Authority
      (Game|SpawnActorfromClass "/Game/_Main/AI/Troll/Projectile_Vomit.Projectile_Vomit_C" (Transformation|GetWorldTransform (Variables|Default|GetVomitSpawn)) "AlwaysSpawn" self (Variables|Default|GetRangeAttackDamage) 0))))

(event EventChasePlayer
  (if (CallFunction|FGetCombatState)
    (bind _length (CallFunction|FPickAttack (Transformation|GetDistanceTo self (CallFunction|FGetPlayerTarget))))
    (Utilities|FlowControl|Delay (+ _length 0.5))
    (CallFunction|ChasePlayer)
    (AI|AIMoveTo self "0, 0, 0" (CallFunction|FGetPlayerTarget) 5e+01 true
      (:OnSuccess
        (CallFunction|RunAttackChoices)))))

(event EventDoSphereOverlap
  (bind _returnvalue (Transformation|GetActorLocation))
  (bind _returnvalue_2 (Transformation|GetActorForwardVector))
  (bind _returnvalue_3 (Transformation|GetActorLocation))
  (bind _returnvalue_4 (Transformation|GetActorForwardVector))
  (bind _returnvalue_5 (* _returnvalue_2 2e+02))
  (bind _returnvalue_6 (* _returnvalue_4 2e+02))
  (bind _returnvalue_7 (+ _returnvalue_3 _returnvalue_6))
  (bind _returnvalue_8 (+ _returnvalue _returnvalue_5))
  (Networking|SwitchHasAuthority
    (:Authority
      (switch Utilities|FlowControl|Switch|SwitchonE_AIAttackTypes (CallFunction|FGetAttackType)
        (:NewEnumerator1
          ;[1 1 1] Heavy attack & knock-back affect
          (bind _outactors (Collision|SphereOverlapActors _returnvalue_8 1e+02 (Utilities|Array|MakeArray "ObjectTypeQuery3") 0 (Utilities|Array|MakeArray self)))
          (Rendering|Debug|DrawDebugSphere _returnvalue_8 1e+02 12 "(R=1.000000,G=0.104167,B=0.104167,A=1.000000)" 2.0 1.0)
          (for _array_element _outactors
            (if (Actor|ActorHasTag _array_element "Player")
              (CallFunction|FGetDamage _array_element)
              (Character|LaunchCharacter (.AsCharacter (Utilities|Casting|CastToCharacter _array_element)) (* (Math|Vector|MakeVector (.X (Math|Vector|BreakVector (Math|Vector|GetUnitDirection(Vector) (Transformation|GetActorLocation (.AsCharacter (Utilities|Casting|CastToCharacter _array_element))) (Transformation|GetActorLocation)))) (.Y (Math|Vector|BreakVector (Math|Vector|GetUnitDirection(Vector) (Transformation|GetActorLocation (.AsCharacter (Utilities|Casting|CastToCharacter _array_element))) (Transformation|GetActorLocation)))) (+ (.Z (Math|Vector|BreakVector (Math|Vector|GetUnitDirection(Vector) (Transformation|GetActorLocation (.AsCharacter (Utilities|Casting|CastToCharacter _array_element))) (Transformation|GetActorLocation)))) 1.0)) 9e+02) false false))))
        (:NewEnumerator3
          ;[1 1 1] Charge Attack
          (bind _outactors_2 (Collision|SphereOverlapActors _returnvalue_7 1.5e+02 (Utilities|Array|MakeArray "ObjectTypeQuery3") 0 (Utilities|Array|MakeArray self)))
          (Rendering|Debug|DrawDebugSphere _returnvalue_7 1e+02 12 "(R=1.000000,G=0.104167,B=0.104167,A=1.000000)" 2.0 1.0)
          (for _array_element_2 _outactors_2
            (if (Actor|ActorHasTag _array_element_2 "Player")
              (CallFunction|FGetDamage _array_element_2)
              (Character|LaunchCharacter (.AsCharacter (Utilities|Casting|CastToCharacter _array_element_2)) (* (Math|Vector|MakeVector (.X (Math|Vector|BreakVector (Math|Vector|GetUnitDirection(Vector) (Transformation|GetActorLocation (.AsCharacter (Utilities|Casting|CastToCharacter _array_element_2))) (Transformation|GetActorLocation)))) (.Y (Math|Vector|BreakVector (Math|Vector|GetUnitDirection(Vector) (Transformation|GetActorLocation (.AsCharacter (Utilities|Casting|CastToCharacter _array_element_2))) (Transformation|GetActorLocation)))) (+ (.Z (Math|Vector|BreakVector (Math|Vector|GetUnitDirection(Vector) (Transformation|GetActorLocation (.AsCharacter (Utilities|Casting|CastToCharacter _array_element_2))) (Transformation|GetActorLocation)))) 1.0)) 9e+02) false false))))))))

(fn ConstructionScript
  (|CallParentFunction))