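; BP_HumanCharacter is the player-controlled human character, handling camera-relative movement, look, and networked sprint and roll.
; Sprint sets walk speed locally and on the server through an RPC, while the Sprinting RepNotify messages the anim instance.
; Rolling goes through a server event to a multicast that plays the roll montage and messages the anim instance, with montage completion clearing the state through the server.
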(event Custom|Server_ToggleSprint
  (params (State :type Boolean))
  ;[1 1 1] Sprint
  (CallFunction|FSprintSwitch State))

(event Custom|Server_Rolling
  (params (Rolling :type Boolean))
  ;[1 1 1] Rolling
  (if Rolling
    (Variables|Default|SetRolling true)
    (CallFunction|MultiRolling (Variables|Character|GetMesh) "/Game/_Main/Player/PlayerRoll_Montage.PlayerRoll_Montage" true)
    (else
      (Variables|Default|SetRolling false)
      (CallFunction|MultiRolling 0 "/Game/_Main/Player/PlayerRoll_Montage.PlayerRoll_Montage" false))))

(event Custom|Multi_Rolling
  (params (SkeletalMeshComponent :type Skeletal%20Mesh%20Component%20Object%20Reference) (Montage :type Anim%20Montage%20Object%20Reference) (State :type Boolean))
  (bind _mesh (Variables|Character|GetMesh))
  (bind _returnvalue (Components|SkeletalMesh|GetAnimInstance _mesh))
  ;[1 1 1] Rolling
  (if State
    (Class|BPIPlayer|RollingState(Message) _returnvalue true)
    (Animation|Montage|PlayMontage SkeletalMeshComponent Montage
      (:OnCompleted
        (CallFunction|ServerRolling false)))
    (else
      (Class|BPIPlayer|RollingState(Message) _returnvalue false))))

(event Input|ActionEvents|InputActionSprint
  (params (Key :type Key%20Structure :default "None"))
  ;[1 1 1] Sprint
  (:Pressed
    (CallFunction|FSprintSwitch true))
  (:Released
    (CallFunction|FSprintSwitch false)))

(event Input|ActionEvents|InputActionRolling
  (params (Key :type Key%20Structure :default "None"))
  ;[1 1 1] Rolling
  (:Pressed
    (if (not (Variables|Default|GetRolling))
      (CallFunction|ServerRolling true))))

(event Input|AxisEvents|InputAxisTurn
  (params (AxisValue :type Float%20%28single-precision%29))
  ;[1 1 1] Movement
  (Pawn|Input|AddControllerYawInput AxisValue))

(event Input|AxisEvents|InputAxisLookUp
  (params (AxisValue :type Float%20%28single-precision%29))
  ;[1 1 1] Movement
  (Pawn|Input|AddControllerPitchInput AxisValue))

(event Input|AxisEvents|InputAxisMoveForward
  (params (AxisValue :type Float%20%28single-precision%29))
  ;[1 1 1] Movement
  (Pawn|Input|AddMovementInput (Math|Vector|GetForwardVector (Math|Rotator|MakeRotator 0.0 0.0 (.Yaw (Math|Rotator|BreakRotator (Pawn|GetControlRotation :!class /Script/Engine.Pawn))))) AxisValue false))

(event Input|AxisEvents|InputAxisMoveRight
  (params (AxisValue :type Float%20%28single-precision%29))
  ;[1 1 1] Movement
  (Pawn|Input|AddMovementInput (Math|Vector|GetRightVector (Math|Rotator|MakeRotator 0.0 0.0 (.Yaw (Math|Rotator|BreakRotator (Pawn|GetControlRotation :!class /Script/Engine.Pawn))))) AxisValue false))

(fn ConstructionScript
  (|CallParentFunction))

(fn FSprintSwitch
  (params (SprintState :type Boolean))
  (bind _charactermovement (Variables|Character|GetCharacterMovement))
  (bind _charactermovement_2 (Variables|Character|GetCharacterMovement))
  (LocalVariables|SetLocalSprint SprintState)
  (Networking|SwitchHasAuthority
    (:Authority
      (if (LocalVariables|GetLocalSprint)
        (Variables|/Script/Engine.CharacterMovementComponent|SetMaxWalkSpeed _charactermovement (Variables|Default|GetSprintSpeed))
        (Variables|Default|SetSprinting true)
        (else
          (Variables|/Script/Engine.CharacterMovementComponent|SetMaxWalkSpeed _charactermovement (Variables|Default|GetJogSpeed))
          (Variables|Default|SetSprinting false)))
      (return))
    (:Remote
      (CallFunction|ServerToggleSprint (LocalVariables|GetLocalSprint))
      (if (LocalVariables|GetLocalSprint)
        (Variables|/Script/Engine.CharacterMovementComponent|SetMaxWalkSpeed _charactermovement_2 (Variables|Default|GetSprintSpeed))
        (else
          (Variables|/Script/Engine.CharacterMovementComponent|SetMaxWalkSpeed _charactermovement_2 (Variables|Default|GetJogSpeed))))
      (return))))

(fn OnRepSprinting
  (bind _mesh (Variables|Character|GetMesh))
  (bind _returnvalue (Components|SkeletalMesh|GetAnimInstance _mesh))
  (if (Variables|Default|GetSprinting)
    (Class|BPIPlayer|SprintState(Message) _returnvalue true)
    (else
      (Class|BPIPlayer|SprintState(Message) _returnvalue false))))