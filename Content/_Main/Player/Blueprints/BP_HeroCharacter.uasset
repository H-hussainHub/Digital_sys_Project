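; BP_HeroCharacter is the networked player character, with movement, sprinting, rolling, a noise-making whistle distraction, melee combat and gear pickup.
; Input routes actions through server events, multicasts play roll and attack montages, and RepNotifies handle sprint animation, gear socket attachment and death.
; Light attacks apply damage through an authority-only sphere overlap, while heavy attack input has no handling.
; Interface messages update the anim instance and controller UI.
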(event Custom|Server_ToggleSprint
  (params (State :type Boolean))
  ;[1 1 1] Sprint
  (Server|FSprintSwitch State))

(event Custom|Server_Rolling
  (params (Rolling :type Boolean))
  ;[1 1 1] Rolling
  (if Rolling
    (Variables|Default|SetRolling true)
    (CallFunction|MultiRolling (Variables|Character|GetMesh) "/Game/_Main/Player/Animation/PlayerRoll_Montage.PlayerRoll_Montage" true)
    (else
      (Variables|Default|SetRolling false)
      (CallFunction|MultiRolling 0 0 false))))

(event Custom|Multi_Rolling
  (params (Mesh :type Skeletal%20Mesh%20Component%20Object%20Reference) (Montage :type Anim%20Montage%20Object%20Reference) (State :type Boolean))
  (bind _returnvalue (Components|SkeletalMesh|GetAnimInstance (Variables|Character|GetMesh)))
  ;[1 1 1] Rolling
  (if true
    (Class|INTHeroAnimBP|RollingState(Message) _returnvalue true)
    (Animation|Montage|PlayMontage Mesh Montage
      (:OnCompleted
        (CallFunction|ServerRolling false)))
    (else
      (Class|INTHeroAnimBP|RollingState(Message) _returnvalue false))))

(event Custom|Server_InteractWithObject
  (Variables|Default|GetOverlappedPickup
    (:then
      (CallFunction|HandlePickup))
    (:else)))

(event Custom|Multi-PlayMontage
  (params (InSkeletalMeshComponent :type Skeletal%20Mesh%20Component%20Object%20Reference) (MontageToPlay :type Anim%20Montage%20Object%20Reference) (StartingSection :type Name))
  ;[1 1 1] Light & Heavy Attack
  (Animation|Montage|PlayMontage InSkeletalMeshComponent MontageToPlay 1.0 0.0 StartingSection
    (:OnCompleted
      _)
    (:OnInterrupted
      _))
  (CallFunction|ServerEndAttack))

(event Custom|Server_EndAttack
  ;[1 1 1] Light & Heavy Attack
  (Variables|Attacking|SetCurrentlyAttacking false))

(event Custom|Server_TryToActivateAbility
  (params (Attacks :type E_PlayerAttacks%20Enum :default "NewEnumerator0"))
  ;[1 1 1] Light & Heavy Attack
  (if (and (not (Variables|Attacking|GetCurrentlyAttacking)) (not (Variables|Default|GetRolling)))
    (switch Utilities|FlowControl|Switch|SwitchonE_PlayerAttacks Attacks
      (:NewEnumerator0
        (Variables|Attacking|SetCurrentlyAttacking true)
        (CallFunction|Multi-PlayMontage (Variables|Character|GetMesh) "/Game/_Main/Player/Animation/LightAttack_Montage.LightAttack_Montage" "None")))))

(event Custom|HandlePickup
  (bind _overlappedpickup (Variables|Default|GetOverlappedPickup))
  ;[1 1 1] Handles pickup objects
  (bind _pickuptype (Class|INTPickups|GetPickupType(Message) (Variables|Default|GetOverlappedPickup)))
  (switch Utilities|FlowControl|Switch|SwitchonE_itemTypes _pickuptype
    (:NewEnumerator1
      (Variables|Inventory|GetEquippedWeapon
        (:then)
        (:else
          (Server|FEquipWeapon _overlappedpickup))))
    (:NewEnumerator2
      (Variables|Inventory|GetEquippedHelmet
        (:then)
        (:else
          (Server|FEquipHelmet _overlappedpickup))))
    (:NewEnumerator7
      (Variables|Inventory|GetEquippedShield
        (:then)
        (:else
          (Server|FEquipShield _overlappedpickup))))))

(event EventSetPickupInfo
  (params (PickupActor :type BP%20Base%20Pickup%20Object%20Reference) (Overlapping :type Boolean))
  (bind _returnvalue (Pawn|GetController))
  ;[1 1 1] Display Pickup Name When Overlapping
  (if Overlapping
    (bind _output_get (Variables|Default|SetOverlappedPickup PickupActor))
    (Class|INTPlayerController|ShowPickupName(Message) _returnvalue true (.PickupName (Utilities|Struct|BreakS_PickupInfo (Variables|/Game/_Main/Pickups/BP_BasePickup.BP_BasePickup_C|GetPickupInfo _output_get))))
    (else
      (Variables|Default|SetOverlappedPickup 0)
      (Class|INTPlayerController|ShowPickupName(Message) _returnvalue false))))

(event EventLightAttack
  (Networking|SwitchHasAuthority
    (:Authority
      (bind (_outactors _returnvalue) (Collision|SphereOverlapActors (+ (* (Transformation|GetActorForwardVector) 1.3e+02) (Transformation|GetActorLocation)) 8e+01 (Utilities|Array|MakeArray "ObjectTypeQuery3") "/Game/_Main/BaseClasses/BP_CharacterBase.BP_CharacterBase_C" (Utilities|Array|MakeArray self)))
      (if _returnvalue
        (for _array_element _outactors
          (Game|Damage|ApplyDamage _array_element (.Damage (Utilities|Struct|BreakS_PickupInfo (Variables|/Game/_Main/Pickups/BP_BasePickup.BP_BasePickup_C|GetPickupInfo (Variables|Inventory|GetEquippedWeapon)))) 0 self "/Script/Engine.DamageType"))))))

(event Game|Damage|EventAnyDamage
  (params (Damage :type Float%20%28single-precision%29) (DamageType :type Damage%20Type%20Object%20Reference) (InstigatedBy :type Controller%20Object%20Reference) (DamageCauser :type Actor%20Object%20Reference))
  (bind _playerstats (Variables|Default|GetPlayerStats))
  (bind _structout (Utilities|Struct|SetmembersinS_PlayerStats _playerstats (- (.CurrentHealth (Utilities|Struct|BreakS_PlayerStats _playerstats)) Damage)))
  (Class|INTPlayerController|UpdateHealthUI(Message) (Pawn|GetController) (/ (.CurrentHealth (Utilities|Struct|BreakS_PlayerStats _structout)) (.MaxHealth (Utilities|Struct|BreakS_PlayerStats _structout))))
  (if (<= (.CurrentHealth (Utilities|Struct|BreakS_PlayerStats _structout)) 0.0)
    (CallFunction|Death)))

(event EventPossessed
  (params (NewController :type Controller%20Object%20Reference))
  (CallFunction|UpdateMovement true))

(event EventDeath
  (if (not (Variables|Default|GetPlayerDead))
    (Variables|Default|SetPlayerDead true)
    (CallFunction|UpdateMovement false)
    (Class|INTPlayerController|DeathScreenUI(Message) (Pawn|GetController))))

(event Input|ActionEvents|InputActionRolling
  (params (Key :type Key%20Structure :default "None"))
  ;[1 1 1] Rolling
  (:Pressed
    (if (not (Variables|Default|GetRolling))
      (CallFunction|ServerRolling true))))

(event Input|ActionEvents|InputActionPrimary
  (params (Key :type Key%20Structure :default "None"))
  ;[1 1 1] Light & Heavy Attack
  (:Pressed
    (if (.EquippedWeapon (Utilities|Struct|BreakS_EquippedItem (Variables|Inventory|GetEquippedItems)))
      (CallFunction|ServerTrytoActivateAbility "NewEnumerator0"))))

(event Input|ActionEvents|InputActionSecondary
  (params (Key :type Key%20Structure :default "None"))
  ;[1 1 1] Light & Heavy Attack
  (:Pressed
    (if (.EquippedWeapon (Utilities|Struct|BreakS_EquippedItem (Variables|Inventory|GetEquippedItems)))
      (CallFunction|ServerTrytoActivateAbility "NewEnumerator1"))))

(event Input|ActionEvents|InputActionInteract
  (params (Key :type Key%20Structure :default "None"))
  (:Pressed
    (CallFunction|ServerInteractwithObject)))

(event Input|ActionEvents|InputActionSprint
  (params (Key :type Key%20Structure :default "None"))
  ;[1 1 1] Sprint
  (:Pressed
    (Server|FSprintSwitch true))
  (:Released
    (Server|FSprintSwitch false)))

(event Input|ActionEvents|InputActionDistract
  (params (Key :type Key%20Structure :default "None"))
  (bind _returnvalue (Transformation|GetActorLocation))
  (:Pressed
    (Audio|PlaySoundatLocation "/Game/_Main/AI/BossAI_Behaviour/Sounds/mixkit-human-whistle-605.mixkit-human-whistle-605" _returnvalue "0, 0, 0" 1.0 1.0 0.0 0 0 0)
    (Class|AISenseHearing|ReportNoiseEvent _returnvalue 1.0 self 0.0 "none")))

(event Input|AxisEvents|InputAxisTurn
  (params (AxisValue :type Float%20%28single-precision%29))
  ;[1 1 1] Movement
  (Pawn|Input|AddControllerYawInput AxisValue))

(event Input|AxisEvents|InputAxisLookUp
  (params (AxisValue :type Float%20%28single-precision%29))
  ;[1 1 1] Movement
  (Pawn|Input|AddControllerPitchInput AxisValue))

(event Input|AxisEvents|InputAxisMoveForward
  (params (AxisValue :type Float%20%28single-precision%29))
  ;[1 1 1] Movement
  (if (Variables|Default|GetCanMove)
    (Pawn|Input|AddMovementInput (Math|Vector|GetForwardVector (Math|Rotator|MakeRotator 0.0 0.0 (.Yaw (Math|Rotator|BreakRotator (Pawn|GetControlRotation :!class /Script/Engine.Pawn))))) AxisValue false)))

(event Input|AxisEvents|InputAxisMoveRight
  (params (AxisValue :type Float%20%28single-precision%29))
  ;[1 1 1] Movement
  (if (Variables|Default|GetCanMove)
    (Pawn|Input|AddMovementInput (Math|Vector|GetRightVector (Math|Rotator|MakeRotator 0.0 0.0 (.Yaw (Math|Rotator|BreakRotator (Pawn|GetControlRotation :!class /Script/Engine.Pawn))))) AxisValue false)))

(fn ConstructionScript
  (|CallParentFunction))

(fn FSprintSwitch
  (params (SprintState :type Boolean))
  (bind _charactermovement (Variables|Character|GetCharacterMovement))
  (bind _charactermovement_2 (Variables|Character|GetCharacterMovement))
  (LocalVariables|SetLocalSprint SprintState)
  (Networking|SwitchHasAuthority
    (:Authority
      (if (LocalVariables|GetLocalSprint)
        (Variables|/Script/Engine.CharacterMovementComponent|SetMaxWalkSpeed _charactermovement_2 (Variables|Default|GetSprintSpeed))
        (Variables|Default|SetSprinting true)
        (else
          (Variables|/Script/Engine.CharacterMovementComponent|SetMaxWalkSpeed _charactermovement_2 (Variables|Default|GetJogSpeed))
          (Variables|Default|SetSprinting false)))
      (return))
    (:Remote
      (CallFunction|ServerToggleSprint (LocalVariables|GetLocalSprint))
      (if (LocalVariables|GetLocalSprint)
        (Variables|/Script/Engine.CharacterMovementComponent|SetMaxWalkSpeed _charactermovement (Variables|Default|GetSprintSpeed))
        (else
          (Variables|/Script/Engine.CharacterMovementComponent|SetMaxWalkSpeed _charactermovement (Variables|Default|GetJogSpeed))))
      (return))))

(fn OnRepSprinting
  (bind _mesh (Variables|Character|GetMesh))
  (bind _returnvalue (Components|SkeletalMesh|GetAnimInstance _mesh))
  (if (Variables|Default|GetSprinting)
    (Class|INTHeroAnimBP|SprintState(Message) _returnvalue true)
    (else
      (Class|INTHeroAnimBP|SprintState(Message) _returnvalue false))))

(fn OnRepEquippedWeapon
  (bind _equippedweapon (Variables|Inventory|GetEquippedWeapon))
  (Transformation|AttachComponentToComponent _equippedweapon (Variables|Character|GetMesh) "Weapon_R" "SnapToTarget" "SnapToTarget" "KeepRelative" true)
  (Class|INTPickups|DisablePhysics(Message) _equippedweapon))

(fn FEquipWeapon
  (params (EquippedWeapon :type BP%20Base%20Pickup%20Object%20Reference))
  (if (not (.EquippedWeapon (Utilities|Struct|BreakS_EquippedItem (Variables|Inventory|GetEquippedItems))))
    (Variables|Inventory|SetEquippedWeapon EquippedWeapon)
    (Utilities|Struct|SetmembersinS_EquippedItem (Variables|Inventory|GetEquippedItems) true)))

(fn OnRepEquippedShield
  (bind _equippedshield (Variables|Inventory|GetEquippedShield))
  (Transformation|AttachComponentToComponent _equippedshield (Variables|Character|GetMesh) "Shield" "SnapToTarget" "SnapToTarget" "KeepRelative" true)
  (Class|INTPickups|DisablePhysics(Message) _equippedshield))

(fn OnRepEquippedHelmet
  (bind _equippedhelmet (Variables|Inventory|GetEquippedHelmet))
  (Transformation|AttachComponentToComponent _equippedhelmet (Variables|Character|GetMesh) "Helmet" "SnapToTarget" "SnapToTarget" "KeepRelative" true)
  (Class|INTPickups|DisablePhysics(Message) _equippedhelmet))

(fn FEquipShield
  (params (EquippedShield :type BP%20Base%20Pickup%20Object%20Reference))
  (if (not (.EquippedShield (Utilities|Struct|BreakS_EquippedItem (Variables|Inventory|GetEquippedItems))))
    (Variables|Inventory|SetEquippedShield EquippedShield)
    (Utilities|Struct|SetmembersinS_EquippedItem (Variables|Inventory|GetEquippedItems) true)))

(fn FEquipHelmet
  (params (EquippedHelmet :type BP%20Base%20Pickup%20Object%20Reference))
  (if (not (Utilities|Struct|BreakS_EquippedItem (Variables|Inventory|GetEquippedItems)))
    (Variables|Inventory|SetEquippedHelmet EquippedHelmet)
    (Utilities|Struct|SetmembersinS_EquippedItem (Variables|Inventory|GetEquippedItems) true)))

(fn OnRepPlayerDead
  (if (Variables|Default|GetPlayerDead)
    (Components|Animation|PlayAnimation (Variables|Character|GetMesh) "/Game/_Main/Player/Animation/Death.Death" false)
    (Collision|SetCollisionProfileName (Variables|Default|GetCapsuleComponent) "RagDoll" true :!class /Script/Engine.PrimitiveComponent)))

(fn IsDead
  (return (Variables|Default|GetPlayerDead)))

(fn UpdateMovement
  (params (CanMove :type Boolean))
  (bind _output_get (Variables|Default|SetCanMove CanMove))
  (return _output_get))